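; Shooter game mode that tracks enemy deaths and prints a victory message once all enemies are killed.
; BeginPlay resets the kill count and counts the BP_Enemy actors in the level as the target.
; A death event increments the count and checks it against that target.
; The loop binding this event to each enemy's OnDeath is disconnected, so nothing in this Blueprint triggers the count.
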(event `self.ReceiveBeginPlay`
  (set `self.KilledEnemy` 0)
  (bind _outactors (`GameplayStatics.GetAllActorsOfClass` "/Game/Blueprints/Characters/Enemies/BP_Enemy.BP_Enemy_C"))
  (set `self.EnemyAmount` (`KismetArrayLibrary.Array_Length` _outactors)))

(event `OnEnemyDeath_Event`
  (bind _output_get (set `self.KilledEnemy` (+ (`self.KilledEnemy`) 1)))
  (if (== (`self.EnemyAmount`) _output_get)
    (`KismetSystemLibrary.PrintString` "VICTORY" true true (struct :`R` 0.093431 :`G` 0.520833 :`B` 0.058274 :`A` 1.0) 180.0)))

(fn `UserConstructionScript`)