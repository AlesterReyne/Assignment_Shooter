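; Base weapon Blueprint that handles shooting, ammo, reloading and activation for the player's weapons.
; The IA_Shoot input, while active, spends ammo and spawns a BP_Bullet with its Damage at BP_Player's BarrelPivot, or prints a warning when empty.
; Bullets are physics projectiles, launched by an impulse along the pawn's forward vector.
; SetWeaponActive toggles visibility and marks possession on activation; Reload refills ammo to maximum.
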(event `EnhancedInput|/Game/Input/IA_Shoot`
  (params (ActionValue :type Boolean) (ElapsedSeconds :type "Float (double-precision)") (TriggeredSeconds :type "Float (double-precision)") (InputAction :type "InputAction Object Reference" :default "/Game/Input/IA_Shoot.IA_Shoot"))
  (bind _currentammo (`self.CurrentAmmo`))
  (:`Triggered`
    (if (`self.isWeaponActive`)
      (if (> _currentammo 0)
        (`/Engine/EditorBlueprintResources/StandardMacros.DecrementInt` _currentammo
          (:`  `
            (bind _asbp_player (cast `/Game/Blueprints/Characters/BP_Player` (`GameplayStatics.GetPlayerPawn` 0)))
            (bind _returnvalue (`|SpawnActorFromClass` "/Game/Blueprints/Items/Weapons/BP_Bullet.BP_Bullet_C" (`KismetMathLibrary.MakeTransform` (`self.K2_GetComponentLocation` (`/Game/Blueprints/Characters/BP_Player.Barrel Pivot` _asbp_player))) "Undefined" "MultiplyWithRoot" null (`self.Damage`) null))
            (bind _sphere (`/Game/Blueprints/Items/Weapons/BP_Bullet.Sphere` _returnvalue))
            (`PrimitiveComponent.SetSimulatePhysics` _sphere true)
            (`PrimitiveComponent.AddImpulse` _sphere (* (`Actor.GetActorForwardVector` (`GameplayStatics.GetPlayerPawn` 0)) 10000.0) "None" false)))
        (else
          (`KismetSystemLibrary.PrintString` "No bullets!"))))))

(fn `Reload`
  (set `self.CurrentAmmo` (`self.MaxAmmo`)))

(fn `SetWeaponActive`
  (params (isActive :type Boolean))
  (`self.SetVisibility` isActive true)
  (set `self.isWeaponActive` isActive)
  (if isActive
    (set `self.isWeaponInPlayerPossesion` true)))