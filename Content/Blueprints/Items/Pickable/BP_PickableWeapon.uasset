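; Pickable weapon item that activates a weapon on the player when touched.
; Overlap by a BP_Player that is the first player's pawn triggers OnPickup, then destroys the actor.
; OnPickup extends the parent pickup logic by passing WeaponType to the player's ActivateWeapon.
; Tick sets the actor's yaw from an incremented DeltaSeconds value.
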(event `self.ReceiveTick`
  (params (DeltaSeconds :type "Float (single-precision)"))
  (bind _result (`/Engine/EditorBlueprintResources/StandardMacros.IncrementFloat` DeltaSeconds)
    (:`  `
      (`self.K2_SetActorRotation` (`KismetMathLibrary.MakeRotator` 0.0 0.0 _result)))))

(event `self.ReceiveActorBeginOverlap`
  (params (OtherActor :type "Actor Object Reference"))
  (cast `/Game/Blueprints/Characters/BP_Player` OtherActor)
  (if (== null (`GameplayStatics.GetPlayerPawn` 0))
    (`self.OnPickup`)
    (`self.K2_DestroyActor`)))

(fn `OnPickup`
  (`parent.OnPickup`)
  (bind _asbp_player (cast `/Game/Blueprints/Characters/BP_Player` (`GameplayStatics.GetPlayerPawn` 0)))
  (`/Game/Blueprints/Characters/BP_Player.ActivateWeapon` _asbp_player (`self.WeaponType`)))

(fn `UserConstructionScript`
  (`parent.UserConstructionScript`))