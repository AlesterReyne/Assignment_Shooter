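; Enemy character with a Tick-driven state machine that patrols random BP_PatrolPoint actors, watches a spotted player, then chases.
; Sight requires the player in range and hit by a debug-drawn forward line trace.
; Timers gate the chase and tire the enemy, which ignores the player until its next patrol point; catching the player only prints game over.
; TakeDamage reduces health, calling OnDeath and destroying the actor at zero.
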(event `self.ReceiveBeginPlay`
  (set `self.CurrentHealth` (`self.MaxHealth`))
  (set `self.NotTired` true)
  (set `self.EnemyState` "NewEnumerator0")
  (`self.GetRandomPatrolPoint`))

(event `self.ReceiveTick`
  (params (DeltaSeconds :type "Float (single-precision)"))
  (bind _returnvalue (`GameplayStatics.GetPlayerPawn` 0))
  (bind _currentpatrolpoint (`self.CurrentPatrolPoint`))
  (set `self.CurrentFrameTimeDelta` DeltaSeconds)
  (bind _seeplayer (`self.CanSeePlayer`))
  (if (and _seeplayer (`self.NotTired`) (`|EnumInequality` (`self.EnemyState`) "NewEnumerator2"))
    (set `self.EnemyState` "NewEnumerator1"))
  (switch `/Game/Blueprints/Characters/Enemies/E_EnemyState` (`self.EnemyState`)
    (:`NewEnumerator0`
      ; Patrol
      (set `self.AttackingPlayerTimer` 0.0)
      (set `self.FindingPlayerTimer` 0.0)
      (`self.RotateToTarget` _currentpatrolpoint)
      (`self.AddMovementInput` (`KismetMathLibrary.Normal` (- (`self.K2_GetActorLocation` _currentpatrolpoint) (`self.K2_GetActorLocation`))) (`self.Speed`))
      (bind _isinrange (`self.isInRange` _currentpatrolpoint 200.0))
      (if _isinrange
        (set `self.NotTired` true)
        (`self.GetRandomPatrolPoint`)))
    (:`NewEnumerator1`
      ; Looking for Player
      (`self.RotateToTarget` _returnvalue)
      (bind _output_get (set `self.FindingPlayerTimer` (+ (`self.CurrentFrameTimeDelta`) (`self.FindingPlayerTimer`))))
      (if (>= _output_get (`self.TimeToLookPlayer`))
        (bind _seeplayer_2 (`self.CanSeePlayer`))
        (if _seeplayer_2
          (set `self.EnemyState` "NewEnumerator2")
          (else
            (set `self.EnemyState` "NewEnumerator0")))))
    (:`NewEnumerator2`
      ; Attack
      (bind _seeplayer_3 (`self.CanSeePlayer`))
      (if _seeplayer_3
        (`self.RotateToTarget` _returnvalue)
        (`self.AddMovementInput` (`KismetMathLibrary.Normal` (- (`self.K2_GetActorLocation` _returnvalue) (`self.K2_GetActorLocation`))) 0.5)
        (bind _isinrange_2 (`self.isInRange` _returnvalue 1.0))
        (if _isinrange_2
          (`KismetSystemLibrary.PrintString` "GAME OVER!" true true (struct :`R` 0.5 :`A` 1.0) 30.0)
          (else
            (bind _output_get_2 (set `self.AttackingPlayerTimer` (+ (`self.AttackingPlayerTimer`) (`self.CurrentFrameTimeDelta`))))
            (if (>= _output_get_2 (`self.TimeToAttackPlayer`))
              (set `self.NotTired` false)
              (set `self.EnemyState` "NewEnumerator0"))))
        (else
          (set `self.FindingPlayerTimer` 0.0)
          (set `self.EnemyState` "NewEnumerator1"))))))

(fn `CanSeePlayer`
  (returns (SeePlayer :type Boolean))
  (bind _returnvalue (`GameplayStatics.GetPlayerPawn` 0))
  (bind _returnvalue_2 (`self.K2_GetActorLocation`))
  (bind _isinrange (`self.isInRange` _returnvalue 1000.0))
  (bind _outhit (`KismetSystemLibrary.LineTraceSingleByProfile` :`Start` _returnvalue_2 :`End` (+ _returnvalue_2 (* (`self.GetActorForwardVector`) 10000.0)) :`ProfileName` "Pawn" :`DrawDebugType` "ForDuration"))
  (return (and _isinrange (== (`.HitActor` (`GameplayStatics.BreakHitResult` _outhit)) _returnvalue))))

(fn `GetRandomPatrolPoint`
  (bind _outactors (`GameplayStatics.GetAllActorsOfClass` "/Game/Blueprints/Characters/Enemies/BP_PatrolPoint.BP_PatrolPoint_C"))
  (set `self.CurrentPatrolPoint` (`|GetArrayItem` _outactors (`KismetMathLibrary.RandomIntegerInRange` 0 (- (`KismetArrayLibrary.Array_Length` _outactors) 1)))))

(fn `isInRange`
  (params (Object :type "Actor Object Reference") (Range :type "Float (double-precision)"))
  (returns (isInRange :type Boolean))
  (return (<= (`self.GetDistanceTo` Object) Range)))

(fn `RotateToTarget`
  (params (Target :type "Actor Object Reference"))
  (bind (_returnvalue_roll _returnvalue_pitch _returnvalue_yaw) (`KismetMathLibrary.BreakRotator` (`self.K2_GetActorRotation`)))
  (bind (_returnvalue_roll_2 _returnvalue_pitch_2 _returnvalue_yaw_2) (`KismetMathLibrary.BreakRotator` (`KismetMathLibrary.NormalizedDeltaRotator` (`KismetMathLibrary.FindLookAtRotation` (`self.K2_GetActorLocation`) (`self.K2_GetActorLocation` Target)) (`self.K2_GetActorRotation`))))
  (`self.K2_SetActorRotation` (`KismetMathLibrary.MakeRotator` 0.0 0.0 (+ _returnvalue_yaw_2 _returnvalue_yaw))))

(fn `TakeDamage`
  (params (Damage :type Integer))
  (bind _output_get (set `self.CurrentHealth` (- (`self.CurrentHealth`) Damage)))
  (if (<= _output_get 0)
    (`self.OnDeath`)
    (`self.K2_DestroyActor`)
    (else
      (`KismetSystemLibrary.PrintString` (`KismetStringLibrary.Concat_StrStr` "Enemy Health: " (`KismetStringLibrary.Conv_IntToString` _output_get)) true true (struct :`G` 0.66 :`B` 1.0 :`A` 1.0) 5.0))))

(fn `UserConstructionScript`)