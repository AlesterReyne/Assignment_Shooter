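; BP_Player is the player character, handling Enhanced Input movement, camera look and weapon switching.
; BeginPlay adds the mapping context, gathers all BP_WeaponBase components and deactivates them.
; Switching cycles an index through every weapon, activating that one only if possessed, so unowned slots leave none active.
; ActivateWeapon selects by type without an ownership check and syncs the index, while ReloadWeapon passes ammo to the given weapon.
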(event `EnhancedInput|/Game/Input/IA_SwitchWeapon`
  (params (ActionValue :type Boolean) (ElapsedSeconds :type "Float (double-precision)") (TriggeredSeconds :type "Float (double-precision)") (InputAction :type "InputAction Object Reference" :default "/Game/Input/IA_SwitchWeapon.IA_SwitchWeapon"))
  ; Weapon Switching
  (:`Triggered`
    (bind _output_get (set `self.WeaponIndex` (mod (+ (`self.WeaponIndex`) 1) (`KismetArrayLibrary.Array_Length` (`self.Weapons`)))))
    (for (_array_element _array_index) (`self.K2_GetComponentsByClass` "/Game/Blueprints/Items/Weapons/BP_WeaponBase.BP_WeaponBase_C")
      (`/Game/Blueprints/Items/Weapons/BP_WeaponBase.SetWeaponActive` _array_element (and (`/Game/Blueprints/Items/Weapons/BP_WeaponBase.isWeaponInPlayerPossesion` _array_element) (== _array_index _output_get))))))

(event `self.ReceiveBeginPlay`
  ; Initialize Weapons in the Start
  (set `self.Barrel Edge` (`self.Barrel Pivot`))
  (`self.SetupInput`)
  (for _array_element (`self.K2_GetComponentsByClass` "/Game/Blueprints/Items/Weapons/BP_WeaponBase.BP_WeaponBase_C")
    (`KismetArrayLibrary.Array_Add` (`self.Weapons`) _array_element)
    (`/Game/Blueprints/Items/Weapons/BP_WeaponBase.SetWeaponActive` _array_element false)))

(event `EnhancedInput|/Game/Input/IA_MoveForward`
  (params (ActionValue :type "Float (double-precision)") (ElapsedSeconds :type "Float (double-precision)") (TriggeredSeconds :type "Float (double-precision)") (InputAction :type "InputAction Object Reference" :default "/Game/Input/IA_MoveForward.IA_MoveForward"))
  ; Movement
  (:`Triggered`
    (`self.AddMovementInput` (`KismetMathLibrary.GetForwardVector` (`self.GetControlRotation`)) ActionValue)))

(event `EnhancedInput|/Game/Input/IA_MoveRight`
  (params (ActionValue :type "Float (double-precision)") (ElapsedSeconds :type "Float (double-precision)") (TriggeredSeconds :type "Float (double-precision)") (InputAction :type "InputAction Object Reference" :default "/Game/Input/IA_MoveRight.IA_MoveRight"))
  ; Movement
  (:`Triggered`
    (`self.AddMovementInput` (`KismetMathLibrary.GetRightVector` (`self.GetControlRotation`)) ActionValue)))

(event `EnhancedInput|/Game/Input/IA_Turn`
  (params (ActionValue :type "Float (double-precision)") (ElapsedSeconds :type "Float (double-precision)") (TriggeredSeconds :type "Float (double-precision)") (InputAction :type "InputAction Object Reference" :default "/Game/Input/IA_Turn.IA_Turn"))
  ; Camera
  (:`Triggered`
    (`self.AddControllerYawInput` ActionValue)))

(event `EnhancedInput|/Game/Input/IA_LookUp`
  (params (ActionValue :type "Float (double-precision)") (ElapsedSeconds :type "Float (double-precision)") (TriggeredSeconds :type "Float (double-precision)") (InputAction :type "InputAction Object Reference" :default "/Game/Input/IA_LookUp.IA_LookUp"))
  ; Camera
  (:`Triggered`
    (`self.AddControllerPitchInput` ActionValue)))

(fn `ActivateWeapon`
  (params (`Weapon Type` :type "/Game/Blueprints/Items/Weapons/E_WeaponType Enum" :default "NewEnumerator0"))
  (for (_array_element _array_index) (`self.K2_GetComponentsByClass` "/Game/Blueprints/Items/Weapons/BP_WeaponBase.BP_WeaponBase_C")
    (bind _returnvalue (`|EnumEquality` `Weapon Type` (`/Game/Blueprints/Items/Weapons/BP_WeaponBase.WeaponType` _array_element)))
    (`/Game/Blueprints/Items/Weapons/BP_WeaponBase.SetWeaponActive` _array_element _returnvalue)
    (if _returnvalue
      (set `self.WeaponIndex` _array_index))))

(fn `ReloadWeapon`
  (params (Weapon :type "/Game/Blueprints/Items/Weapons/BP_WeaponBase Object Reference") (Ammo :type Integer))
  (`/Game/Blueprints/Items/Weapons/BP_WeaponBase.Reload` Weapon Ammo))

(fn `SetupInput`
  (`EnhancedInputSubsystemInterface.AddMappingContext` (pcsubsystem `EnhancedInputLocalPlayerSubsystem` (`GameplayStatics.GetPlayerController` 0)) "/Game/Input/IMC_Player.IMC_Player" 0 (struct)))

(fn `UserConstructionScript`)